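; Game mode that procedurally spawns loot at BeginPlay, placing a BP_ItemGroup at each location in DT_ItemGroupLocations.
; Each group gets a weighted-random item count, random transforms from the group, non-repeating item types and an ID from that type's probability table.
; A BP_TestItem is spawned per pick.
; Weighting comes from data tables, filling arrays with each entry repeated by its Percent and drawing one at random.
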(event EventBeginPlay
  (CallFunction|GenerateItems))

(event EventTick
  (params (DeltaSeconds :type Float%20%28single-precision%29)))

(fn ConstructionScript)

(fn GenerateItems
  ;[0.15 0.15 0.15 0.5] 위치를 지정한 아이템 그룹들을 스폰
  ;;[0.15 0.15 0.15 0.5] 데이터 테이블의 전체 로우 네임 가져오기
  (bind _outrownames (DataTable|GetDataTableRowNames "/Game/Blueprints/Datas/DataTable/ItemGeneration/DT_ItemGroupLocations.DT_ItemGroupLocations"))
  (for _array_element _outrownames
    (bind _returnvalue (Utilities|GetDataTableRow "/Game/Blueprints/Datas/DataTable/ItemGeneration/DT_ItemGroupLocations.DT_ItemGroupLocations" _array_element)
      (:then
        (bind _returnvalue_2 (Game|SpawnActorfromClass "/Game/Blueprints/Items/BP_ItemGroup.BP_ItemGroup_C" (Math|Transform|MakeTransform (.location _returnvalue) "0, 0, 0" "1.000000,1.000000,1.000000") "Undefined" "MultiplyWithRoot" 0 0))
        (LocalVariables|SetItemGroupRef _returnvalue_2)
        (Utilities|Array|Clear (LocalVariables|GetItemTypeArray))
        ;[0.15 0.15 0.15 0.5] 아이템 그룹에 생성될 랜덤 아이템 개수 정하기
        (bind _number (CallFunction|RandomItemNumber))
        (LocalVariables|SetSpawnTransforms (Default|GetRandomTransform (LocalVariables|GetItemGroupRef) _number))
        (for _index (range 1 _number)
          (bind _itemtype (CallFunction|RandomItemType :!label _label))
          ;[0.15 0.15 0.15 0.5] 랜덤 아이템 중복 방지
          (if (== (Utilities|Array|FindItem (LocalVariables|GetItemTypeArray) _itemtype) -1)
            (Utilities|Array|Add (LocalVariables|GetItemTypeArray) _itemtype)
            (else
              (goto _label))))
        (for _array_element_2 (LocalVariables|GetItemTypeArray)
          (bind _spawnitem (CallFunction|RandomItemId _array_element_2))
          (Utilities|Array|Add (LocalVariables|GetSpawnItemArray) _spawnitem))
        (for (_array_element_3 _array_index) (LocalVariables|GetSpawnItemArray)
          (LocalVariables|SetItemType (.itemtype _array_element_3))
          (LocalVariables|SetSpawnId (.id _array_element_3))
          (Game|SpawnActorfromClass "/Game/Blueprints/BP_TestItem.BP_TestItem_C" (Utilities|Array|Get(acopy) (LocalVariables|GetSpawnTransforms) _array_index) "Undefined" "MultiplyWithRoot" 0 0))
        (Utilities|Array|Clear (LocalVariables|GetSpawnItemArray))))))

(fn RandomItemNumber
  ;[0.15 0.15 0.15 0.5] 데이터 테이블에서 각 숫자가 나올 확률 가져오기
  (bind _outrownames (DataTable|GetDataTableRowNames "/Game/Blueprints/Datas/DataTable/ItemGeneration/DT_NumberProbabilities.DT_NumberProbabilities"))
  (for _array_element _outrownames
    (bind _returnvalue (Utilities|GetDataTableRow "/Game/Blueprints/Datas/DataTable/ItemGeneration/DT_NumberProbabilities.DT_NumberProbabilities" _array_element)
      (:then
        ;[0.15 0.15 0.15 0.5] 각 숫자를 퍼센트만큼 배열에 채워주기
        (for _index (range 1 (.percent _returnvalue))
          ;;[0.15 0.15 0.15 0.5] 3*30 / 4*40 / 5*30
          (Utilities|Array|Add (LocalVariables|GetNumberArray) (.number _returnvalue))))))
  (return (.OutItem (Utilities|Array|Random (LocalVariables|GetNumberArray)))))

(fn RandomItemType
  ;[0.15 0.15 0.15 0.5] 데이터 테이블에서 각 숫자가 나올 확률 가져오기
  (bind _outrownames (DataTable|GetDataTableRowNames "/Game/Blueprints/Datas/DataTable/ItemGeneration/DT_ItemTypeProbabillity.DT_ItemTypeProbabillity"))
  (for _array_element _outrownames
    (bind _returnvalue (Utilities|GetDataTableRow "/Game/Blueprints/Datas/DataTable/ItemGeneration/DT_ItemTypeProbabillity.DT_ItemTypeProbabillity" _array_element)
      (:then
        ;[0.15 0.15 0.15 0.5] 각 숫자를 퍼센트만큼 배열에 채워주기
        (for _index (range 1 (.percent _returnvalue))
          (Utilities|Array|Add (LocalVariables|GetItemTypeArray) (.itemtype _returnvalue))))))
  (return (.OutItem (Utilities|Array|Random (LocalVariables|GetItemTypeArray)))))

(fn RandomItemId
  (params (ItemType :type E_ItemType%20Enum :default "NewEnumerator0"))
  (bind _returnvalue (Utilities|Select :Index ItemType :NewEnumerator0 "/Game/Blueprints/Datas/DataTable/ItemGeneration/DT_WeaponProbabillity.DT_WeaponProbabillity" :NewEnumerator1 "/Game/Blueprints/Datas/DataTable/ItemGeneration/DT_AccessariesProbabillity.DT_AccessariesProbabillity" :NewEnumerator2 "/Game/Blueprints/Datas/DataTable/ItemGeneration/DT_AmmoProbabillity.DT_AmmoProbabillity" :NewEnumerator3 "/Game/Blueprints/Datas/DataTable/ItemGeneration/DT_HealthProbabillity.DT_HealthProbabillity" :NewEnumerator4 "/Game/Blueprints/Datas/DataTable/ItemGeneration/DT_BoostProbabillity.DT_BoostProbabillity" :NewEnumerator5 "/Game/Blueprints/Datas/DataTable/ItemGeneration/DT_HelmetProbabillity.DT_HelmetProbabillity" :NewEnumerator6 "/Game/Blueprints/Datas/DataTable/ItemGeneration/DT_VestProbabillity.DT_VestProbabillity" :NewEnumerator7 "/Game/Blueprints/Datas/DataTable/ItemGeneration/DT_BackPackProbabillity.DT_BackPackProbabillity"))
  (Utilities|FlowControl|Sequence
    (:then_0
      (bind _outrownames (DataTable|GetDataTableRowNames _returnvalue))
      (for _array_element _outrownames
        (bind _returnvalue_2 (Utilities|GetDataTableRow _returnvalue _array_element)
          (:then
            (for _index (range 1 (Utilities|Struct|BreakST_ItemProbabillity _returnvalue_2))
              (Utilities|Array|Add (LocalVariables|GetItemArray) (Utilities|Struct|MakeST_SpawnItem ItemType _array_element)))))))
    (:then_1
      (return (.OutItem (Utilities|Array|Random (LocalVariables|GetItemArray)))))))